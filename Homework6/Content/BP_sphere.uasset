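; BP_sphere is an actor that moves in a straight line and bounces off whatever blocks it.
; Each tick it does a swept world offset along Direction, scaled by Speed and delta time.
; On a blocking hit it cuts Speed by a fixed fraction, clamped to MinSpeed, reflects Direction about the hit normal and prints the new speed.
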(event EventTick
  (params (DeltaSeconds :type Float%20%28single-precision%29))
  (bind _min_speed (Variables|Default|Getmin%20Speed))
  (bind _sweephitresult (Transformation|AddActorWorldOffset (* DeltaSeconds (* (Variables|Default|Getdirection) (Variables|Default|Getspeed))) true))
  (if (.bBlockingHit (Collision|BreakHitResult _sweephitresult))
    (Utilities|FlowControl|Sequence
      (:then_0
        (if (>= (- (Variables|Default|Getspeed) (* (Variables|Default|Getspeed) 0.2)) _min_speed)
          (Variables|Default|Setspeed (- (Variables|Default|Getspeed) (* (Variables|Default|Getspeed) 0.2)))
          (else
            (Variables|Default|Setspeed _min_speed))))
      (:then_1
        (Variables|Default|Setdirection (Math|Vector|GetReflectionVector (Variables|Default|Getdirection) (.Normal (Collision|BreakHitResult _sweephitresult))))
        (Development|PrintString (Utilities|String|ToString(Float) (Variables|Default|Getspeed)))))))

(event EventBeginPlay)

(event Collision|EventActorBeginOverlap
  (params (OtherActor :type Actor%20Object%20Reference)))

(fn ConstructionScript)